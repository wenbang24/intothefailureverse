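; A countdown timer actor that shows minutes and seconds on a text render until time runs out, then changes a cube.
; Tick runs a one-second Delay that decrements Seconds and rolls over into Minutes.
; At zero it calls SetStaticMesh on the Cube with no mesh, blanks the text and sets a Gone flag that stops further display updates.
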(event EventTick
  (params (DeltaSeconds :type Float%20%28single-precision%29))
  (Utilities|FlowControl|Sequence
    (:then_0
      (Utilities|FlowControl|Delay 1.0)
      (if (== (Variables|Default|GetSeconds) 0)
        (if (not (== (Variables|Default|GetMinutes) 0))
          (Variables|Default|SetSeconds 59)
          (Variables|Default|SetMinutes (- (Variables|Default|GetMinutes) 1)))
        (else
          (Variables|Default|SetSeconds (- (Variables|Default|GetSeconds) 1)))))
    (:then_1
      (if (and (== (Variables|Default|GetSeconds) 0) (== (Variables|Default|GetMinutes) 0))
        (Components|StaticMesh|SetStaticMesh (Variables|Default|GetCube) 0)
        (Rendering|Components|TextRender|SetText (Variables|Default|GetTextRender) (Utilities|Text|ToText(String) ""))
        (Variables|Default|Setgone true)))
    (:then_2
      (if (not (Variables|Default|Getgone))
        (Rendering|Components|TextRender|SetText (Variables|Default|GetTextRender) (Utilities|Text|ToText(String) (Utilities|String|Append (Utilities|String|ToString(Integer) (Variables|Default|GetMinutes)) ":" (Utilities|String|ToString(Integer) (Variables|Default|GetSeconds)))))))))

(fn ConstructionScript)