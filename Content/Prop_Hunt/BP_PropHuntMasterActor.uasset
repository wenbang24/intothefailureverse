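; Base prop actor for a Prop Hunt mode, holding a configurable static mesh and uniform scale.
; The construction script applies the NewMesh and MeshScale variables to the PropMesh component.
; GetMesh exposes the component's current mesh and the scale value to callers, and the event graph has no active logic.
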(event EventBeginPlay)

(event Collision|EventActorBeginOverlap
  (params (OtherActor :type Actor%20Object%20Reference)))

(event EventTick
  (params (DeltaSeconds :type Float%20%28single-precision%29)))

(fn ConstructionScript
  (bind _mesh_scale (Variables|Default|GetMesh%20Scale))
  (Transformation|SetRelativeScale3D (Variables|Default|GetPropMesh) (Math|Vector|MakeVector _mesh_scale _mesh_scale _mesh_scale))
  (Components|StaticMesh|SetStaticMesh (Variables|Default|GetPropMesh) (Variables|Default|GetNew%20Mesh)))

(fn GetMesh
  (return (Variables|/Script/Engine.StaticMeshComponent|GetStaticMesh (Variables|Default|GetPropMesh)) (Variables|Default|GetMesh%20Scale)))